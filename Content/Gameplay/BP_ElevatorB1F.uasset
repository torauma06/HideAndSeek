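; BP_ElevatorB1F is a B1F elevator with two sliding doors and a number-entry UI for the first-person player.
; While the doors are closed, entering its box shows a text prompt and enables input, so E toggles the escape number widget and cursor.
; Leaving disables input and clears all widgets.
; The OpenElevator event, not called within this Blueprint, slides both doors via nested timelines, marks them open and hides the prompt.
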(event `self.Box.OnComponentBeginOverlap`
  (params (OverlappedComponent :type "PrimitiveComponent Object Reference") (OtherActor :type "Actor Object Reference") (OtherComp :type "PrimitiveComponent Object Reference") (OtherBodyIndex :type Integer) (bFromSweep :type Boolean) (SweepResult :type "HitResult Structure (by ref)"))
  (cast `/Game/Gameplay/BP_FirstPerson` OtherActor)
  (if (not (`self.IsDoorOpen`))
    (`self.EnableInput` (`GameplayStatics.GetPlayerController` 0))
    (`SceneComponent.SetVisibility` (`self.TextRender`) true false)))

(event `Open Elevator`
  (bind (_direction _leftdooropen) (`Timeline|Left Door Timeline`)
    (:`Update`
      (`SceneComponent.K2_SetRelativeLocation` (`self.LeftDoor1`) _leftdooropen false false)
      (bind (_direction_2 _rightdooropen) (`Timeline|Right Door Timeline`)
        (:`Update`
          (`SceneComponent.K2_SetRelativeLocation` (`self.RightDoor1`) _rightdooropen false false)
          (set `self.IsDoorOpen` true)
          (`SceneComponent.SetVisibility` (`self.TextRender`) false false))))))

(event `self.Box.OnComponentEndOverlap`
  (params (OverlappedComponent :type "PrimitiveComponent Object Reference") (OtherActor :type "Actor Object Reference") (OtherComp :type "PrimitiveComponent Object Reference") (OtherBodyIndex :type Integer))
  (bind _returnvalue (`GameplayStatics.GetPlayerController` 0))
  (cast `/Game/Gameplay/BP_FirstPerson` OtherActor)
  (`self.DisableInput` (`GameplayStatics.GetPlayerController` 0))
  (`SceneComponent.SetVisibility` (`self.TextRender`) false false)
  (`WidgetLayoutLibrary.RemoveAllWidgets` :!label _label)
  (`WidgetBlueprintLibrary.SetInputMode_GameOnly` _returnvalue)
  (set `PlayerController.bShowMouseCursor` false _returnvalue))

(event `Key|E`
  (params (Key :type "Key Structure"))
  (bind _returnvalue (`GameplayStatics.GetPlayerController` 0))
  (:`Pressed`
    (`/Engine/EditorBlueprintResources/StandardMacros.FlipFlop`
      (:`A`
        (bind _returnvalue_2 (`|CreateWidget` "/Game/UI/Number_UI_B1F_ESCAPE_01.Number_UI_B1F_ESCAPE_01_C"))
        (`UserWidget.AddToViewport` _returnvalue_2 0)
        (`WidgetBlueprintLibrary.SetInputMode_GameAndUIEx` _returnvalue null)
        (set `PlayerController.bShowMouseCursor` true _returnvalue))
      (:`B`
        (goto _label)))))

(fn `UserConstructionScript`)