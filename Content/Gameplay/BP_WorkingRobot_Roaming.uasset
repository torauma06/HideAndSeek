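; Working robot enemy that spots pawns through PawnSensing and chases the player, with roaming only stubbed out.
; On seeing any pawn, it records whether that pawn is the player, swaps a mesh material to the visor warning material and starts an AI move toward the player regardless.
; A retriggerable delay follows but drives nothing, and the Roaming event calls AI MoveTo without a pawn or target.
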(event `self.PawnSensing.OnSeePawn`
  (params (Pawn :type "Pawn Object Reference"))
  (set `self.IsSensingPlayer?` (== Pawn (`GameplayStatics.GetPlayerCharacter` 0)))
  (`self.ChangeWarninglight`)
  (`KismetSystemLibrary.PrintString` "Find")
  (`|ExecutionSequence`
    (:`then_0`
      (`|AIMoveTo` self (0.0 0.0 0.0) (`GameplayStatics.GetPlayerPawn` 0)
        (:`then`
          (`KismetSystemLibrary.PrintString` "Chasing"))))
    (:`then_1`
      (`KismetSystemLibrary.RetriggerableDelay` 1.0))))

(event `Roaming`
  (`|AIMoveTo` null (0.0 0.0 0.0) null))

(fn `ChangeWarninglight`
  (`PrimitiveComponent.SetMaterial` (`self.Mesh`) 1 "/Game/SciFi_Robot/MATERIALS/VISOR/VISOR_MAT.VISOR_MAT"))

(fn `UserConstructionScript`)