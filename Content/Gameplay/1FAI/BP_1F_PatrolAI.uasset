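; BP_1F_PatrolAI is a patrol AI threat that warns the player by heartbeat and triggers death on contact.
; Overlapping the HeartBeats volume opens a heartbeat media source on the Heartbeat player, and leaving it closes playback.
; Player overlap with the PlayerDie volume shows the UI_YouDie widget and stops the heartbeat.
; The end-overlap event skips the player check, so any actor leaving silences it; the graph contains no patrol logic.
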(event `self.HeartBeats.OnComponentBeginOverlap`
  (params (OverlappedComponent :type "PrimitiveComponent Object Reference") (OtherActor :type "Actor Object Reference") (OtherComp :type "PrimitiveComponent Object Reference") (OtherBodyIndex :type Integer) (bFromSweep :type Boolean) (SweepResult :type "HitResult Structure (by ref)"))
  ;[1 1 1] HeartBeats
  (if (== OtherActor (`GameplayStatics.GetPlayerCharacter` 0))
    (`MediaPlayer.OpenSource` (`self.heartbeat`) "/Game/Sound/369017__patobottos__heartbeats-61.369017__patobottos__heartbeats-61")))

(event `self.HeartBeats.OnComponentEndOverlap`
  (params (OverlappedComponent :type "PrimitiveComponent Object Reference") (OtherActor :type "Actor Object Reference") (OtherComp :type "PrimitiveComponent Object Reference") (OtherBodyIndex :type Integer))
  ;[1 1 1] HeartBeats
  (`MediaPlayer.Close` (`self.heartbeat`)))

(event `self.PlayerDie.OnComponentBeginOverlap`
  (params (OverlappedComponent :type "PrimitiveComponent Object Reference") (OtherActor :type "Actor Object Reference") (OtherComp :type "PrimitiveComponent Object Reference") (OtherBodyIndex :type Integer) (bFromSweep :type Boolean) (SweepResult :type "HitResult Structure (by ref)"))
  (if (== OtherActor (`GameplayStatics.GetPlayerCharacter` 0))
    (bind _returnvalue (`|CreateWidget` "/Game/UI/UI_YouDie.UI_YouDie_C"))
    (`UserWidget.AddToViewport` _returnvalue 0)
    (`MediaPlayer.Close` (`self.heartbeat`))))

(fn `UserConstructionScript`)