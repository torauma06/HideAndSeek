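; BP_basePanel is a gimmick panel that shows and hides a readable note as a screen widget.
; TogglePickup checks the IsReading flag to choose between PickupNote and PulldownNote.
; PickupNote creates a fresh NewWidgetBlueprint and adds it to the viewport, while PulldownNote removes it from its parent, each updating the flag.
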(event `Toggle Pickup`
  (if (`self.IsReading`)
    (`self.Pulldown Note`)
    (else
      (`self.Pickup Note`))))

(event `Pickup Note`
  (bind _returnvalue (`|CreateWidget` "/Game/GimickObject/GimickPanel/NewWidgetBlueprint.NewWidgetBlueprint_C"))
  (`UserWidget.AddToViewport` _returnvalue 0)
  (set `self.IsReading` true))

(event `Pulldown Note`
  (`Widget.RemoveFromParent` (stale `Pickup Note` _returnvalue))
  (set `self.IsReading` false))

(fn `UserConstructionScript`)